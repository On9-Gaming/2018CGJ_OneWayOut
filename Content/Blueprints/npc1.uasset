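; NPC that wanders randomly and counts as a player win the moment it takes any damage.
; Tick runs through a one-second Delay, then sends its controller to a random reachable navmesh point within a radius of itself via SimpleMoveToLocation.
; AnyDamage calls PlayerWin on the MyGameMode cached at BeginPlay, spawns an enlarged steam particle effect and destroys the NPC.
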(event `self.ReceiveBeginPlay`
  (bind _asmy_game_mode (cast `/Game/Blueprints/MyGameMode` (`GameplayStatics.GetGameMode`)))
  (set `self.my game mode` _asmy_game_mode))

(event `self.ReceiveTick`
  (params (DeltaSeconds :type "Float (single-precision)"))
  (bind (_randomlocation _returnvalue) (`NavigationSystem.K2_GetRandomReachablePointInRadius` (`self.K2_GetActorLocation`) 2000.0))
  (`KismetSystemLibrary.Delay` 1.0)
  (if _returnvalue
    (`NavigationSystem.SimpleMoveToLocation` (`self.GetController`) _randomlocation)))

(event `self.ReceiveAnyDamage`
  (params (Damage :type "Float (single-precision)") (DamageType :type "DamageType Object Reference") (InstigatedBy :type "Controller Object Reference") (DamageCauser :type "Actor Object Reference"))
  (`/Game/Blueprints/MyGameMode.player win` (`self.my game mode`))
  (`GameplayStatics.SpawnEmitterAtLocation` "/Game/GameJamKit/Effects/Steam/P_SubtleSteam_Rise_Slow.P_SubtleSteam_Rise_Slow" (`self.K2_GetActorLocation`) (struct) (3.0 3.0 3.0))
  (`self.K2_DestroyActor`))

(fn `UserConstructionScript`)