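; GassCan1 is a gas can pickup for VR that the player collects by touching it with either motion controller.
; BeginPlay casts and caches MyGameMode.
; When its Box is overlapped, it compares the other actor to the left and right controllers of the first MotionControllerPawn found in the level.
; On a match it increments the game mode's GassCanCount and destroys itself.
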(event `self.ReceiveBeginPlay`
  (bind _asmy_game_mode (cast `/Game/Blueprints/MyGameMode` (`GameplayStatics.GetGameMode`)))
  (set `self.MyGmaeMode` _asmy_game_mode))

(event `self.Box.OnComponentBeginOverlap`
  (params (OverlappedComponent :type "PrimitiveComponent Object Reference") (OtherActor :type "Actor Object Reference") (OtherComp :type "PrimitiveComponent Object Reference") (OtherBodyIndex :type Integer) (bFromSweep :type Boolean) (SweepResult :type "HitResult Structure (by ref)"))
  (bind _mygmaemode (`self.MyGmaeMode`))
  (bind _outactors (`GameplayStatics.GetAllActorsOfClass` "/Game/Blueprints/MotionControllerPawn.MotionControllerPawn_C"))
  (bind _output (`|GetArrayItem` _outactors))
  (if (and (!= OtherActor self) (or (== OtherActor (`/Game/Blueprints/MotionControllerPawn.RightController` _output)) (== OtherActor (`/Game/Blueprints/MotionControllerPawn.LeftController` _output))))
    (set `/Game/Blueprints/MyGameMode.GassCanCount` (+ (`/Game/Blueprints/MyGameMode.GassCanCount` _mygmaemode) 1) _mygmaemode)
    (`self.K2_DestroyActor`)))

(fn `UserConstructionScript`)