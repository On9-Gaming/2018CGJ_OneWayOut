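; Car Blueprint that acts as a trigger for the player's win check.
; On BeginPlay it casts the current game mode to MyGameMode and caches the reference.
; When the player pawn, provided it is not the car itself, begins overlapping the Box component, it calls CheckPlayerWin on that game mode, which handles the win logic.
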(event `self.ReceiveBeginPlay`
  (bind _asmy_game_mode (cast `/Game/Blueprints/MyGameMode` (`GameplayStatics.GetGameMode`)))
  (set `self.my game mode` _asmy_game_mode))

(event `self.Box.OnComponentBeginOverlap`
  (params (OverlappedComponent :type "PrimitiveComponent Object Reference") (OtherActor :type "Actor Object Reference") (OtherComp :type "PrimitiveComponent Object Reference") (OtherBodyIndex :type Integer) (bFromSweep :type Boolean) (SweepResult :type "HitResult Structure (by ref)"))
  (if (and (== OtherActor (`GameplayStatics.GetPlayerPawn` 0)) (!= OtherActor self))
    (`/Game/Blueprints/MyGameMode.check player win` (`self.my game mode`))))

(fn `UserConstructionScript`)