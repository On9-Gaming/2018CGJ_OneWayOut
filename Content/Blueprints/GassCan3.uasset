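; GassCan3 is a gas can pickup that adds to a running count when something touches it.
; BeginPlay casts the current game mode to MyGameMode and caches the reference.
; When any other actor overlaps its Box component, it increments GassCanCount on that game mode and destroys itself, with no check that the actor is the player.
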(event `self.ReceiveBeginPlay`
  (bind _asmy_game_mode (cast `/Game/Blueprints/MyGameMode` (`GameplayStatics.GetGameMode`)))
  (set `self.MyGameMode` _asmy_game_mode))

(event `self.Box.OnComponentBeginOverlap`
  (params (OverlappedComponent :type "PrimitiveComponent Object Reference") (OtherActor :type "Actor Object Reference") (OtherComp :type "PrimitiveComponent Object Reference") (OtherBodyIndex :type Integer) (bFromSweep :type Boolean) (SweepResult :type "HitResult Structure (by ref)"))
  (bind _mygamemode (`self.MyGameMode`))
  (if (!= OtherActor self)
    (set `/Game/Blueprints/MyGameMode.GassCanCount` (+ (`/Game/Blueprints/MyGameMode.GassCanCount` _mygamemode) 1) _mygamemode)
    (`self.K2_DestroyActor`)))

(fn `UserConstructionScript`)